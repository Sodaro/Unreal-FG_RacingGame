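; BP_PowerupPickup is a powerup pickup actor that so far only animates its Cube component, with no overlap or collection logic.
; Tick spins the cube in world yaw using a macro that scales delta time for a frame-rate-independent rate.
; Sine waves of game time bob its relative height and drive a clamped X/Y scale pulse, leaving Z scale fixed.
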(event EventBeginPlay)

(event Collision|EventActorBeginOverlap
  (params (OtherActor :type Actor%20Object%20Reference)))

(event EventTick
  (params (DeltaSeconds :type Float%20%28single-precision%29))
  (bind _returnvalue (Utilities|Time|GetTimeSeconds))
  (bind _returnvalue_2 (Math|Trig|Sin(Radians) _returnvalue))
  (bind _returnvalue_3 (* _returnvalue_2 1e+01))
  (bind _returnvalue_4 (- 1e+01 _returnvalue_3))
  (bind _returnvalue_5 (Math|Float|Clamp(Float) _returnvalue_4 1.0 2.0))
  (Transformation|AddWorldRotation (Variables|Default|GetCube) (Math|Rotator|MakeRotator 0.0 0.0 (.dA (Utilities|NewMacro0 DeltaSeconds 9e+01 45.0))) false false)
  (Transformation|SetRelativeLocation (Variables|Default|GetCube) (Math|Vector|MakeVector 0.0 0.0 (* _returnvalue_2 5e+01)) false false)
  (Transformation|SetRelativeScale3D (Variables|Default|GetCube) (Math|Vector|MakeVector _returnvalue_5 _returnvalue_5 1.0)))

(fn ConstructionScript)